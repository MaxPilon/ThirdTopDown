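; BP_EnemyBase is a base enemy that chases a player target, attacks in melee and dies when its health runs out.
; ChasePlayer moves it with AIMoveTo, and on arrival Attack damages player characters inside a sphere overlap at AttackPoint.
; A hit leads back into the chase after a short delay, while a miss ends the loop.
; AnyDamage lowers Health, and Death stops movement and destroys the actor.
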(event Custom|Death
  ;[1 1 1] Death
  (Pawn|Components|CharacterMovement|DisableMovement (Variables|Character|GetCharacterMovement))
  (AI|Navigation|StopMovement (Pawn|GetController))
  (Actor|DestroyActor))

(event Custom|ChasePlayer
  (params (Target :type Pawn%20Object%20Reference))
  ;[1 1 1] Chase Player
  (Variables|Default|SetPlayerTarget Target)
  (AI|AIMoveTo self "0, 0, 0" Target 5.0 false
    (:OnSuccess
      (CallFunction|Attack))))

(event Custom|Attack
  ;[1 1 1] Attack Player
  (bind _outactors (Collision|SphereOverlapActors (Transformation|GetWorldLocation (Variables|Default|GetAttackPoint)) 8e+01 (Utilities|Array|MakeArray "ObjectTypeQuery3") "/Game/Blueprints/BP_PlayerCharacter.BP_PlayerCharacter_C"))
  (for _array_element _outactors
    (Game|Damage|ApplyDamage _array_element (Variables|Default|GetBase%20Damage) 0 self "/Script/Engine.DamageType")
    (Utilities|FlowControl|Delay 0.3)
    (CallFunction|ChasePlayer (Variables|Default|GetPlayerTarget))))

(event Game|Damage|EventAnyDamage
  (params (Damage :type Float%20%28single-precision%29) (DamageType :type Damage%20Type%20Object%20Reference) (InstigatedBy :type Controller%20Object%20Reference) (DamageCauser :type Actor%20Object%20Reference))
  ;[1 1 1] Receive Damage
  (Variables|Default|SetHealth (- (Variables|Default|GetHealth) Damage))
  (if (<= (Variables|Default|GetHealth) 0.0)
    (CallFunction|Death)))

(fn ConstructionScript)