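; Player character Blueprint with axis-driven movement, mouse yaw turning, a dash and projectile firing.
; Dash temporarily boosts walk speed and acceleration while a timeline pushes movement along the capsule's forward vector, then stops, restores normal values and runs a cooldown.
; Fire spawns a scaled BP_Projectile at the Spawner, aimed along the actor's forward vector.
; An unused LaunchCharacter-based dash variant remains disconnected in the graph.
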(event Input|ActionEvents|InputActionDash
  (params (Key :type Key%20Structure :default "None"))
  ;[1 1 1] NOT USED Dash Version_2 (More simple but limited)
)

(event Input|ActionEvents|InputActionDash
  (params (Key :type Key%20Structure :default "None"))
  (bind _charactermovement (Variables|Character|GetCharacterMovement))
  (bind _charactermovement_2 (Variables|Character|GetCharacterMovement))
  ;[0.2195 0.6242 1] MOVEMENT
  ;;[1 1 1] Dash
  (:Pressed
    (if (Variables|Default|GetCanDash?)
      ;;;[1 1 1] How Fast
      (Variables|/Script/Engine.CharacterMovementComponent|SetMaxAcceleration _charactermovement_2 5e+04)
      (Variables|/Script/Engine.CharacterMovementComponent|SetMaxWalkSpeed _charactermovement_2 3e+03)
      ;;;[1 1 1] How long
      (Timeline|Dash PlayFromStart
        (:Update
          (Pawn|Input|AddMovementInput (Math|Vector|GetForwardVector (Variables|Collision|GetCapsuleComponent)) 1.0 false))
        (:Finished
          ;;;[1 1 1] Set speed back to normal after Dash
          (Components|Movement|StopMovementImmediately _charactermovement)
          (Variables|/Script/Engine.CharacterMovementComponent|SetMaxAcceleration _charactermovement 2048.0)
          (Variables|/Script/Engine.CharacterMovementComponent|SetMaxWalkSpeed _charactermovement 6e+02)
          ;;;[1 1 1] Delay/CoolDown
          (Variables|Default|SetCanDash? false)
          (Utilities|FlowControl|Delay 1.0)
          (Variables|Default|SetCanDash? true))))))

(event Input|ActionEvents|InputActionFire
  (params (Key :type Key%20Structure :default "None"))
  (:Pressed
    (Game|SpawnActorfromClass "/Game/Blueprints/BP_Projectile.BP_Projectile_C" (Math|Transform|MakeTransform (Transformation|GetWorldLocation (Variables|Default|GetSpawner)) (Math|Conversions|RotationFromXVector (Transformation|GetActorForwardVector)) "0.500000,0.200000,0.200000") "Undefined" 0 0)))

(event Input|AxisEvents|InputAxisForward_Backward
  (params (AxisValue :type Float%20%28single-precision%29))
  ;[0.2195 0.6242 1] MOVEMENT
  ;;[1 1 1] Forward_Backward_Left_Right
  (Pawn|Input|AddMovementInput (Math|Vector|GetForwardVector (Pawn|GetControlRotation :!class /Script/Engine.Pawn)) AxisValue false))

(event Input|AxisEvents|InputAxisLeft_Right
  (params (AxisValue :type Float%20%28single-precision%29))
  ;[0.2195 0.6242 1] MOVEMENT
  ;;[1 1 1] Forward_Backward_Left_Right
  (Pawn|Input|AddMovementInput (Math|Vector|GetRightVector (Pawn|GetControlRotation :!class /Script/Engine.Pawn)) AxisValue false))

(event Input|AxisEvents|InputAxisRotate_Left_Right
  (params (AxisValue :type Float%20%28single-precision%29))
  ;[0.2195 0.6242 1] MOVEMENT
  ;;[1 1 1] Rotation Mouse
  (Pawn|Input|AddControllerYawInput AxisValue))

(fn ConstructionScript)