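; Wave manager that runs endless-style enemy waves in the arena, with a short countdown before each.
; On BeginPlay it sorts spawn points by enemy type, then a looping timer counts down to the wave.
; Each wave reads its data table row by wave number and spawns enemies at random matching points.
; It polls every second until all spawned enemies are invalid, then plays a sound and advances the wave.
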(event Custom|Start%20Countdown
  ;[1 1 1] Countdown
  (bind _returnvalue (Utilities|Time|SetTimerbyEvent (delegate Custom|Count) 1.0 true))
  (Variables|Default|SetTime 3))

(event Custom|Count
  ;[1 1 1] Countdown
  ;;[1 1 1] If have widget, remove this
  (Development|PrintString (Utilities|String|ToString(Integer) (Variables|Default|GetTime)))
  (if (== (Variables|Default|GetTime) 0)
    (Utilities|Time|ClearandInvalidateTimerbyHandle (stale Custom|Start%20Countdown _returnvalue))
    (CallFunction|BeginWave)
    (else
      (Math|Integer|DecrementInt (Variables|Default|GetTime)))))

(event Custom|Begin%20Wave
  ;[1 1 1] Spawn Enemies for Wave
  ;;[1 1 1] Get all enemy info from this wave
  (bind _returnvalue (Utilities|GetDataTableRow (Variables|Default|GetEnemyDataTable) (Utilities|String|StringToName (Utilities|String|ToString(Integer) (Variables|Default|GetWaveNumber))))
    (:then
      (for _array_element (Utilities|Struct|BreakWaveInfo _returnvalue)
        ;;[1 1 1] Double click for info on SpawnPoint
        (CallFunction|SpawnEnemies _array_element))
      (CallFunction|StartCheckingifEnemiesAreDead))
    (:RowNotFound
      (Development|PrintString "Couldn't find row for wave Data"))))

(event Custom|Start%20Checking%20If%20Enemies%20Are%20Dead
  ;[1 1 1] Check if enemies are dead and start new wave
  (bind _are_dead_1 (CallFunction|CheckifAllEnemiesDead :!label _label))
  (if _are_dead_1
    ;;[1 1 1] Sound/Screen Between Waves
    (Audio|SpawnSound2D "/Game/StarterContent/Audio/Explosion01.Explosion01" 1.0 1.0 0.0 0)
    (Math|Integer|IncrementInt (Variables|Default|GetWaveNumber)
      (:%20%20
        (CallFunction|StartCountdown)))
    (else
      (Utilities|FlowControl|Delay 1.0)
      (goto _label))))

(event EventBeginPlay
  ;[1 1 1] Sort Enemy Spawner References
  (bind _outactors (Actor|GetAllActorsOfClass "/Game/WaveArena/BP_WaveSpwanPoint.BP_WaveSpwanPoint_C"))
  (bind _output_get (Variables|Default|SetEnemySpawnPoints _outactors))
  (for _array_element _output_get
    (switch Utilities|FlowControl|Switch|SwitchonE_EnemyTypes (Variables|/Game/WaveArena/BP_WaveSpwanPoint.BP_WaveSpwanPoint_C|GetSpawnerType _array_element)
      (:NewEnumerator0
        ;;[1 1 1] Enemies
        (Utilities|Array|Add (Variables|Default|GetE_Enemy_01) _array_element))
      (:NewEnumerator1
        (Utilities|Array|Add (Variables|Default|GetE_Enemy_02) _array_element))))
  (CallFunction|StartCountdown))

(fn ConstructionScript)

(fn SpawnEnemies
  (params (EnemyInfo :type Enemy%20Info%20Structure%20%28by%20ref%29))
  (LocalVariables|SetEnemyInfoRef EnemyInfo)
  (LocalVariables|SetCurrentSpawnPoint (Utilities|Select :Index (.EnemyType (Utilities|Struct|BreakEnemyInfo EnemyInfo)) :NewEnumerator0 (Variables|Default|GetE_Enemy_01) :NewEnumerator1 (Variables|Default|GetE_Enemy_02)))
  (for _index (range 1 (.enemynumber (LocalVariables|GetEnemyInfoRef)))
    (bind _returnvalue (Game|SpawnActorfromClass (.enemyclass (LocalVariables|GetEnemyInfoRef)) (Transformation|GetWorldTransform (Variables|/Game/WaveArena/BP_WaveSpwanPoint.BP_WaveSpwanPoint_C|GetBillboard (Utilities|Array|Get(acopy) (LocalVariables|GetCurrentSpawnPoint) (Math|Random|RandomIntegerinRange 0 (Utilities|Array|LastIndex (LocalVariables|GetCurrentSpawnPoint)))))) "AdjustIfPossibleButAlwaysSpawn" 0 0))
    (Utilities|Array|Add (Variables|Default|GetCurrentEnemies) _returnvalue)))

(fn CheckifAllEnemiesDead
  (LocalVariables|SetAre%20Dead? true)
  (for _array_element (Variables|Default|GetCurrentEnemies)
    (Utilities|IsValid _array_element
      (:Is%20Valid
        (LocalVariables|SetAre%20Dead? false))))
  (return (LocalVariables|GetAre%20Dead?)))